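; Blueprint named after a downtown city afternoon asset that records its start location and provides 2D polar coordinate helpers.
; The construction script stores the actor location in StartPosition, which nothing else shown reads.
; ToPolar returns vector length and X divided by length as Angle, a cosine with no arccosine applied.
; FromPolar treats Angle as a true angle, so the two functions are not inverses.
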(fn `FromPolar`
  (params (len :type "Float (double-precision)") (Angle :type "Float (double-precision)"))
  (returns (x :type "Float (double-precision)") (y :type "Float (double-precision)"))
  (return (* len (`KismetMathLibrary.Cos` Angle)) (* len (`KismetMathLibrary.Sin` Angle))))

(fn `ToPolar`
  (params (Coords :type "Vector2D Structure"))
  (returns (len :type "Float (double-precision)") (angle :type "Float (double-precision)"))
  (bind _returnvalue (`KismetMathLibrary.Sqrt` (+ (`KismetMathLibrary.Square` Coords_X) (`KismetMathLibrary.Square` Coords_Y))))
  (return _returnvalue (/ Coords_X _returnvalue)))

(fn `UserConstructionScript`
  (set `self.StartPosition` (`self.K2_GetActorLocation`)))
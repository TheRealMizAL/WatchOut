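; A player pawn that moves with Enhanced Input and turns its control yaw toward the mouse cursor.
; BeginPlay adds the basic mapping context, and Tick aims the yaw at the deprojected mouse world location.
; Movement follows that yaw, plus a random vector scaled by DrunknessLevel for wobble.
; DrunknessLevel resets to zero when movement starts, and the AddDrunk function is an empty stub.
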(event `self.ReceiveBeginPlay`
  (bind _asplayer_controller (cast `PlayerController` (`self.GetController`)))
  (bind _returnvalue (pcsubsystem `EnhancedInputLocalPlayerSubsystem` _asplayer_controller))
  (`/Engine/EditorBlueprintResources/StandardMacros.IsValid` _returnvalue
    (:`Is Valid`
      (`EnhancedInputSubsystemInterface.AddMappingContext` _returnvalue "/Game/Blueprints/Player/Movement/IM_PlayerBasic.IM_PlayerBasic" 0 (struct)))))

(event `EnhancedInput|/Game/Blueprints/Player/Movement/IA_PlayerMove`
  (params (ActionValue :type "Vector2D Structure") (ElapsedSeconds :type "Float (double-precision)") (TriggeredSeconds :type "Float (double-precision)") (InputAction :type "InputAction Object Reference" :default "/Game/Blueprints/Player/Movement/IA_PlayerMove.IA_PlayerMove"))
  (bind (_returnvalue_roll _returnvalue_pitch _returnvalue_yaw) (`KismetMathLibrary.BreakRotator` (`self.GetControlRotation`)))
  (:`Triggered`
    (`self.AddMovementInput` (+ (* ActionValue_X (`KismetMathLibrary.GetForwardVector` (`KismetMathLibrary.MakeRotator` 0.0 0.0 _returnvalue_yaw))) (* (`KismetMathLibrary.GetRightVector` (`KismetMathLibrary.MakeRotator` 0.0 0.0 _returnvalue_yaw)) ActionValue_Y) (* (`self.DrunknessLevel`) (`KismetMathLibrary.RandomUnitVector`)))))
  (:`Started`
    (if true
      (set `self.DrunknessLevel` 0.0))))

(event `self.ReceiveTick`
  (params (DeltaSeconds :type "Float (single-precision)"))
  (bind (_returnvalue_roll _returnvalue_pitch _returnvalue_yaw) (`KismetMathLibrary.BreakRotator` (`KismetMathLibrary.FindLookAtRotation` (`self.K2_GetActorLocation`) (`PlayerController.DeprojectMousePositionToWorld` (`self.GetLocalViewingPlayerController`)))))
  (`|ExecutionSequence`
    (:`then_1`
      (if true
        (`Controller.SetControlRotation` (`GameplayStatics.GetPlayerController` 0) (`KismetMathLibrary.MakeRotator` 0.0 0.0 _returnvalue_yaw))))))

(fn `Add Drunk`
  (params (StartX :type "Float (double-precision)") (StartY :type "Float (double-precision)")))

(fn `UserConstructionScript`)
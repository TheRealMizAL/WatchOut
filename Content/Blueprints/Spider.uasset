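; Spider enemy that chases the player once its PawnSensing spots them, switching its material from a wall look to spider skin.
; Tick calls FollowPlayer, which issues AIMoveTo while SeePlayer is true; the delayed reset to the wall material runs only when the flag is already false.
; Tick also spawns an attached walking sound while the spider moves and destroys it when it stops.
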(event `self.PawnSensing.OnSeePawn`
  (params (Pawn :type "Pawn Object Reference"))
  (cast `/Game/Blueprints/Player/NewPawn` Pawn)
  (set `self.SeePlayer` true)
  (`PrimitiveComponent.SetMaterial` (`self.Mesh`) 0 "/Game/Pawns/Spider/SpiderSkin.SpiderSkin"))

(event `FollowPlayer`
  (if (`self.SeePlayer`)
    (`|AIMoveTo` self (0.0 0.0 0.0) (`GameplayStatics.GetPlayerCharacter` 0))
    (else
      (`KismetSystemLibrary.Delay` 3.0)
      (set `self.SeePlayer` false)
      (`PrimitiveComponent.SetMaterial` (`self.Mesh`) 0 "/Game/Materials/WallDefault.WallDefault"))))

(event `self.ReceiveTick`
  (params (DeltaSeconds :type "Float (single-precision)"))
  (bind _walksoundspawned (`self.WalkSoundSpawned`))
  (`self.FollowPlayer`)
  (if (> (`KismetMathLibrary.VSize` (`self.GetVelocity`)) 0.0)
    (`/Engine/EditorBlueprintResources/StandardMacros.IsValid` _walksoundspawned
      (:`Is Not Valid`
        (bind _returnvalue (`GameplayStatics.SpawnSoundAttached` "/Game/Sounds/SFX/SpiderWalk.SpiderWalk" (`self.CapsuleComponent`) "None" (0.0 0.0 0.0) (struct) "KeepRelativeOffset" false 1.0 1.0 0.0 "/Game/Sounds/SFX/DoorOpeningAttenuation.DoorOpeningAttenuation" null))
        (set `self.WalkSoundSpawned` _returnvalue)))
    (else
      (`/Engine/EditorBlueprintResources/StandardMacros.IsValid` _walksoundspawned
        (:`Is Valid`
          (`AudioComponent.Stop` _walksoundspawned)
          (`ActorComponent.K2_DestroyComponent` _walksoundspawned))))))

(fn `UserConstructionScript`)